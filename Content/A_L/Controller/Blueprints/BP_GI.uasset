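; BP_GI, likely the game instance, switches the player between a standard pawn and a VR pawn.
; Each swap function teleports the target pawn to the current one, offsetting height between floor-level VR origin and character center.
; It then toggles pawn visibility and VR hands, has the first player controller possess the target, and enables or disables the HMD.
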(fn SwaptoVRCtr
  (bind _pawncharacter (Variables|Default|GetPawnCharacter))
  (bind _returnvalue (Transformation|GetActorLocation _pawncharacter))
  (bind (_x _y _z) (Math|Vector|BreakVector _returnvalue))
  (Transformation|SetActorLocation (Variables|Default|GetPawnCharacterVR) (Math|Vector|MakeVector _x _y (- _z 87.5)) false false)
  (Rendering|SetActorHiddenInGame (Variables|Default|GetPawnCharacter) true)
  (Rendering|SetActorHiddenInGame (Variables|Default|GetPawnCharacterVR) false)
  (Default|EnableHand (Variables|Default|GetPawnCharacterVR))
  (Pawn|Possess (Game|GetPlayerController 0) (Variables|Default|GetPawnCharacterVR))
  (Class|HeadMountedDisplayFunctionLibrary|EnableHMD true)
  (Default|EnableHand (Variables|Default|GetPawnCharacterVR)))

(fn SwaptoNorCtr
  (bind _pawncharactervr (Variables|Default|GetPawnCharacterVR))
  (bind _returnvalue (Transformation|GetActorLocation _pawncharactervr))
  (bind (_x _y _z) (Math|Vector|BreakVector _returnvalue))
  (Transformation|SetActorLocation (Variables|Default|GetPawnCharacter) (Math|Vector|MakeVector _x _y (+ _z 87.5)) false false)
  (Rendering|SetActorHiddenInGame (Variables|Default|GetPawnCharacter) false)
  (Rendering|SetActorHiddenInGame (Variables|Default|GetPawnCharacterVR) true)
  (Default|DisableHand (Variables|Default|GetPawnCharacterVR))
  (Pawn|Possess (Game|GetPlayerController 0) (Variables|Default|GetPawnCharacter))
  (Class|HeadMountedDisplayFunctionLibrary|EnableHMD false)
  (Default|DisableHand (Variables|Default|GetPawnCharacterVR)))